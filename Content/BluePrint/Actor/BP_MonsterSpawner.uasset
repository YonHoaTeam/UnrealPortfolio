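; BP_MonsterSpawner is an actor that spawns monsters around its location, automatically on BeginPlay when AutoSpawn is set.
; SpawnMonster loops up to MaxMonsterCount, with an index-scaled Delay inside the loop body before each spawn call.
; Spawns use random 3D offsets within SpawnRadius and are stored in SpawnedMonster.
; GetAliveCount counts the stored monsters that are still valid and not dead.
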(event `self.ReceiveBeginPlay`
  (if (`self.bAutoSpawn`)
    (`self.SpawnMonster`)))

(event `SpawnMonster`
  (for _index (range (`self.MaxMonsterCount`))
    (`KismetSystemLibrary.Delay` (* _index (`self.SpawnDelay`)))
    (bind _returnvalue (`|SpawnActorFromClass` (`self.MonsterClass`) (`KismetMathLibrary.MakeTransform` (+ (`self.K2_GetActorLocation`) (* (`KismetMathLibrary.RandomUnitVector`) (`KismetMathLibrary.RandomFloatInRange` 0.0 (`self.SpawnRadius`))))) "Undefined" "MultiplyWithRoot" null null))
    (`KismetArrayLibrary.Array_Add` (`self.SpawnedMonster`) _returnvalue)))

(fn `GetAliveCount`
  (returns (AliveCount :type Integer))
  (locals (Count :type Integer))
  (set `local.Count` 0)
  (for _array_element (`self.SpawnedMonster`)
    (`/Engine/EditorBlueprintResources/StandardMacros.IsValid` _array_element
      (:`Is Valid`
        (if (not (`/Game/BluePrint/Enemy/BP_EnemyBase.bIsDead` _array_element))
          (bind _result (`/Engine/EditorBlueprintResources/StandardMacros.IncrementInt` (`local.Count`))
            (:`  `
              (set `local.Count` _result)))))))
  (return (`local.Count`)))

(fn `UserConstructionScript`)