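; AI controller for monsters that idle and chase the player's toon character when perceived.
; On possess it starts the monster behavior tree and seeds the blackboard with the spawn location as home, the patrol wait time and an idle state.
; Perception updates set or clear the target actor and switch the state between chase and idle, printing debug strings on each change.
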(event `self.ReceivePossess`
  (params (PossessedPawn :type "Pawn Object Reference"))
  (bind _returnvalue (`AIBlueprintHelperLibrary.GetBlackboard` self))
  (set `self.Possessed Pawn` PossessedPawn)
  (`self.UseBlackboard` "/Game/BluePrint/AI/BB_Monster.BB_Monster")
  (`self.RunBehaviorTree` "/Game/BluePrint/AI/BT_Monster.BT_Monster")
  (`BlackboardComponent.SetValueAsVector` _returnvalue (`self.HomeLocationKey`) (`self.K2_GetActorLocation` (`self.Possessed Pawn`)))
  (`BlackboardComponent.SetValueAsFloat` _returnvalue (`self.PatrolWaitTimeKey`) (`self.PatrolWaitTime`))
  (`BlackboardComponent.SetValueAsEnum` _returnvalue (`self.StateKey`) 0)
  (`KismetSystemLibrary.PrintString` "Idle1"))

(event `self.AIPerception.OnTargetPerceptionUpdated`
  (params (Actor :type "Actor Object Reference") (Stimulus :type "AIStimulus Structure"))
  (bind _returnvalue (`AIBlueprintHelperLibrary.GetBlackboard` self))
  (bind _returnvalue_2 (`AIBlueprintHelperLibrary.GetBlackboard` self))
  (bind _asbp_toon_character (cast `/Game/BluePrint/Character/BP_ToonCharacter` Actor))
  (if (`.bSuccessfullySensed` (break `AIStimulus` Stimulus))
    (`BlackboardComponent.SetValueAsObject` _returnvalue (`self.TargetActorKey`) _asbp_toon_character)
    (`BlackboardComponent.SetValueAsEnum` _returnvalue (`self.StateKey`) 1)
    (`KismetSystemLibrary.PrintString` "Chase")
    (else
      (`BlackboardComponent.SetValueAsObject` _returnvalue_2 (`self.TargetActorKey`) null)
      (`BlackboardComponent.SetValueAsEnum` _returnvalue_2 (`self.StateKey`) 0)
      (`KismetSystemLibrary.PrintString` "Idle2"))))

(fn `UserConstructionScript`)