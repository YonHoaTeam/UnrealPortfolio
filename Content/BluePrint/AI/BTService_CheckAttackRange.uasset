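; Behavior tree service for monster AI that checks whether the target is within attack range.
; Each tick it reads the TargetActor from the Blackboard and measures its distance to the controlled BP_MonsterBasic pawn.
; Within that monster's AttackRange, it writes MonsterEnum to the State key, with no change when out of range.
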(event `self.ReceiveTickAI`
  (params (OwnerController :type "AIController Object Reference") (ControlledPawn :type "Pawn Object Reference") (DeltaSeconds :type "Float (single-precision)"))
  (bind _asactor (cast `Actor` (`BlackboardComponent.GetValueAsObject` (`AIBlueprintHelperLibrary.GetBlackboard` OwnerController) (`self.TargetActor`))))
  (bind _asbp_monster_basic (cast `/Game/BluePrint/Enemy/BP_MonsterBasic` ControlledPawn))
  (if (<= (`KismetMathLibrary.Vector_Distance` (`Actor.K2_GetActorLocation` ControlledPawn) (`Actor.K2_GetActorLocation` _asactor)) (`/Game/BluePrint/Enemy/BP_MonsterBasic.AttackRange` _asbp_monster_basic))
    (`BlackboardComponent.SetValueAsEnum` (`AIBlueprintHelperLibrary.GetBlackboard` OwnerController) (`self.State`) (`self.MonsterEnum`))))