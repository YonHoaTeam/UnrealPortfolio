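; Basic monster enemy Blueprint that sets up its combat stats from data and provides a montage-based attack with a cooldown.
; BeginPlay looks up the DT_MonsterStat row named by MonsterTid to set health, damage, range, cooldown and walk speed, then enables attacking.
; PerformAttack tests CanAttack for equality with not IsDead, clears it, plays AM_EnemyAttack and starts a cooldown timer.
; No damage is applied here.
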(event `self.ReceiveBeginPlay`
  (`parent.ReceiveBeginPlay`)
  (bind _returnvalue (`|GetDataTableRow` "/Game/Data/DT_MonsterStat.DT_MonsterStat" (`KismetStringLibrary.Conv_StringToName` (`KismetStringLibrary.Conv_IntToString` (`self.MonsterTid`))))
    (:`then`
      (bind (_monstertid _maxhp _attackdamage _attackrange _detectionrange _attackcooldown _movespeed) (break `/Game/Data/S_MonsterStat` _returnvalue))
      (set `self.CurrentHP` _maxhp)
      (set `self.MaxHP` _maxhp)
      (set `self.AttackDamage` _attackdamage)
      (set `self.AttackRange` _attackrange)
      (set `self.AttackCooldown` _attackcooldown)
      (set `CharacterMovementComponent.MaxWalkSpeed` _movespeed (`self.CharacterMovement`))
      (set `self.bCanAttack` true))))

(event `ResetCanAttack`
  (set `self.bCanAttack` true))

(fn `PerformAttack`
  (if (== (`self.bCanAttack`) (not (`self.bIsDead`)))
    (set `self.bCanAttack` false)
    (`self.PlayAnimMontage` "/Game/BluePrint/Enemy/AM_EnemyAttack.AM_EnemyAttack")
    (`KismetSystemLibrary.K2_SetTimerDelegate` (`|CreateDelegate` :!event `ResetCanAttack`) (`self.AttackCooldown`))))

(fn `UserConstructionScript`
  (`parent.UserConstructionScript`))