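; Animation notify state that opens and closes an attack check window during montages or animations for enemies and the toon character.
; On begin and end it casts the mesh owner to BP_EnemyBase, falling back to BP_ToonCharacter, and calls that actor's OnAttackCheckStart or OnAttackCheckEnd.
; An IsHeavy flag is passed through to mark heavy attacks, and other owners are ignored.
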(fn `Received_NotifyBegin`
  (params (MeshComp :type "SkeletalMeshComponent Object Reference") (Animation :type "AnimSequenceBase Object Reference") (TotalDuration :type "Float (single-precision)") (EventReference :type "AnimNotifyEventReference Structure (by ref)"))
  (returns (ReturnValue :type Boolean))
  (bind _returnvalue (`ActorComponent.GetOwner` (`local.MeshComp`)))
  (bind _asbp_enemy_base (cast `/Game/BluePrint/Enemy/BP_EnemyBase` _returnvalue)
    (:`then`
      (`/Game/BluePrint/Enemy/BP_EnemyBase.OnAttackCheckStart` _asbp_enemy_base (`self.IsHeavy`))
      (return true))
    (:`CastFailed`
      (bind _asbp_toon_character (cast `/Game/BluePrint/Character/BP_ToonCharacter` _returnvalue)
        (:`then`
          (`/Game/BluePrint/Character/BP_ToonCharacter.OnAttackCheckStart` _asbp_toon_character (`self.IsHeavy`))
          (return true))
        (:`CastFailed`
          (return false))))))

(fn `Received_NotifyEnd`
  (params (MeshComp :type "SkeletalMeshComponent Object Reference") (Animation :type "AnimSequenceBase Object Reference") (EventReference :type "AnimNotifyEventReference Structure (by ref)"))
  (returns (ReturnValue :type Boolean))
  (bind _returnvalue (`ActorComponent.GetOwner` (`local.MeshComp`)))
  (bind _asbp_enemy_base (cast `/Game/BluePrint/Enemy/BP_EnemyBase` _returnvalue)
    (:`then`
      (`/Game/BluePrint/Enemy/BP_EnemyBase.OnAttackCheckEnd` _asbp_enemy_base (`self.IsHeavy`))
      (return true))
    (:`CastFailed`
      (bind _asbp_toon_character (cast `/Game/BluePrint/Character/BP_ToonCharacter` _returnvalue)
        (:`then`
          (`/Game/BluePrint/Character/BP_ToonCharacter.OnAttackCheckEnd` _asbp_toon_character (`self.IsHeavy`))
          (return true))
        (:`CastFailed`
          (return false))))))