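; Base enemy character with health, melee attacks and lock-on state for combat against BP_ToonCharacter.
; Damage points the AI blackboard at the attacker, updates the HP bar widget, then plays a hit reaction or death, which notifies BP_GameMode, refreshes player lock-on and starts a destroy timer.
; Attack-check functions toggle a hitbox that damages the player once per swing.
; Outline meshes follow body and katana through leader pose; InitFromDataTable is an empty stub.
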(event `self.ReceiveBeginPlay`
  (set `self.Tags` (`self.Tags`))
  (set `self.bIsLockOn` false))

(event `self.ReceiveAnyDamage`
  (params (Damage :type "Float (single-precision)") (DamageType :type "DamageType Object Reference") (InstigatedBy :type "Controller Object Reference") (DamageCauser :type "Actor Object Reference"))
  (if (not (`self.bIsDead`))
    (bind _asaicontroller (cast `AIController` (`self.GetController`)))
    (bind _returnvalue (`AIBlueprintHelperLibrary.GetBlackboard` _asaicontroller))
    (`BlackboardComponent.SetValueAsEnum` _returnvalue (`self.StateKey`) (`self.EnemyEnum`))
    (`BlackboardComponent.SetValueAsVector` _returnvalue (`self.TargetLocationKey`) (`self.K2_GetActorLocation` DamageCauser))
    (`BlackboardComponent.SetValueAsObject` _returnvalue (`self.TargetActor`) DamageCauser)
    (set `self.CurrentHP` (`KismetMathLibrary.FClamp` (- (`self.CurrentHP`) Damage) 0.0 (`self.MaxHP`)))
    (bind _aswbp_enemy_hp (cast `/Game/UI/Widgets/WBP_EnemyHP` (`WidgetComponent.GetUserWidgetObject` (`self.HPBarWidget`))))
    (`/Game/UI/Widgets/WBP_EnemyHP.SetHP` _aswbp_enemy_hp (/ (`self.CurrentHP`) (`self.MaxHP`)))
    (if (<= (`self.CurrentHP`) 0.0)
      (`self.Die`)
      (bind _asbp_toon_character (cast `/Game/BluePrint/Character/BP_ToonCharacter` DamageCauser))
      (if (`/Game/BluePrint/Character/BP_ToonCharacter.bIsLockedOn` _asbp_toon_character)
        (`/Game/BluePrint/Character/BP_ToonCharacter.DisableLockOn` _asbp_toon_character)
        (`/Game/BluePrint/Character/BP_ToonCharacter.EnableLockOn` _asbp_toon_character))
      (else
        (`self.PlayAnimMontage` "/Game/BluePrint/Enemy/AM_EnemyHitReact.AM_EnemyHitReact")
        (`NiagaraFunctionLibrary.SpawnSystemAtLocation` "/Game/Niagra/NS_Simple_Burst_Level_1.NS_Simple_Burst_Level_1" (`self.K2_GetActorLocation` self) (`KismetMathLibrary.Conv_VectorToRotator` (`self.GetActorForwardVector` self)))))))

(event `DelayedDestroy`
  (`self.K2_DestroyActor`))

(event `self.AttackHitbox.OnComponentBeginOverlap`
  (params (OverlappedComponent :type "PrimitiveComponent Object Reference") (OtherActor :type "Actor Object Reference") (OtherComp :type "PrimitiveComponent Object Reference") (OtherBodyIndex :type Integer) (bFromSweep :type Boolean) (SweepResult :type "HitResult Structure (by ref)"))
  (if (not (`KismetArrayLibrary.Array_Contains` (`self.HitActorThisSwing`) OtherActor))
    (`KismetArrayLibrary.Array_Add` (`self.HitActorThisSwing`) OtherActor)
    (bind _asbp_toon_character (cast `/Game/BluePrint/Character/BP_ToonCharacter` OtherActor))
    (`GameplayStatics.ApplyDamage` _asbp_toon_character (`self.AttackDamage`) (`self.GetController`) self)))

(event `LockOn`
  (params (IsLocked :type Boolean))
  (set `self.bIsLockOn` IsLocked))

(fn `Die`
  (locals (State :type Name :default "None"))
  (set `self.bIsDead` true)
  (`BlackboardComponent.SetValueAsEnum` (`AIBlueprintHelperLibrary.GetBlackboard` (`AIBlueprintHelperLibrary.GetAIController` self)) (`local.State`) 3)
  (`PrimitiveComponent.SetCollisionEnabled` (`self.CapsuleComponent`) "QueryOnly")
  (`self.PlayAnimMontage` "/Game/BluePrint/Enemy/AM_EnemyDie.AM_EnemyDie")
  (bind _asbp_game_mode (cast `/Game/BluePrint/BP_GameMode` (`GameplayStatics.GetGameMode`)))
  (`/Game/BluePrint/BP_GameMode.OnEnemyKilled` _asbp_game_mode self)
  (`KismetSystemLibrary.K2_SetTimerDelegate` (`|CreateDelegate` :!event `DelayedDestroy`) 1.5))

(fn `InitFromDataTable`
  (return))

(fn `OnAttackCheckEnd`
  (params (IsHeavyAttack :type Boolean))
  (`PrimitiveComponent.SetCollisionEnabled` (`self.AttackHitbox`) "NoCollision")
  (`KismetArrayLibrary.Array_Clear` (`self.HitActorThisSwing`)))

(fn `OnAttackCheckStart`
  (params (IsHeavyAttack :type Boolean))
  (`KismetArrayLibrary.Array_Clear` (`self.HitActorThisSwing`))
  (`PrimitiveComponent.SetCollisionEnabled` (`self.AttackHitbox`) "QueryOnly"))

(fn `UserConstructionScript`
  (`SkinnedMeshComponent.SetLeaderPoseComponent` (`self.Outline`) (`self.Mesh`) false false)
  (`SkinnedMeshComponent.SetLeaderPoseComponent` (`self.KatanaOutline`) (`self.Katana`) false false))