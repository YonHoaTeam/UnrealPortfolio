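; Game mode that tracks a single kill quest and triggers victory when it is completed.
; BeginPlay loads one hardcoded row from DT_Quest as the current quest.
; OnEnemyKilled counts enemies whose MonsterTid matches the quest target; at the target count it shows WBP_Victory, switches to UI-only input, and disables and stops the player character.
; The OnUpdateQuest event is an empty stub.
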(event `self.ReceiveBeginPlay`
  (bind _returnvalue (`|GetDataTableRow` "/Game/Data/DT_Quest.DT_Quest" "30001")
    (:`then`
      (set `self.CurQuest` _returnvalue))))

(event `OnUpdateQuest`
  (params (QuestTid :type Integer)))

(fn `OnEnemyKilled`
  (params (DeadEnemy :type "/Game/BluePrint/Enemy/BP_EnemyBase Object Reference"))
  (bind _returnvalue (`GameplayStatics.GetPlayerCharacter` 0))
  (bind _returnvalue_2 (`GameplayStatics.GetPlayerController` 0))
  (bind (_curquest_texttid _curquest_targettid) (break `/Game/Data/S_Quest` (`self.CurQuest`)))
  (bind (_curquest_texttid_2 _curquest_targettid_2 _curquest_targetcount) (break `/Game/Data/S_Quest` (`self.CurQuest`)))
  (if (== _curquest_targettid (`/Game/BluePrint/Enemy/BP_EnemyBase.MonsterTid` DeadEnemy))
    (bind _output_get (set `self.QuestCount` (+ (`self.QuestCount`) 1)))
    (if (<= _curquest_targetcount _output_get)
      (bind _returnvalue_3 (`|CreateWidget` "/Game/UI/Widgets/WBP_Victory.WBP_Victory_C" _returnvalue_2))
      (`UserWidget.AddToViewport` _returnvalue_3 0)
      (`WidgetBlueprintLibrary.SetInputMode_UIOnlyEx` _returnvalue_2 _returnvalue_3)
      (`self.DisableInput` _returnvalue _returnvalue_2)
      (`MovementComponent.StopMovementImmediately` (`Character.CharacterMovement` _returnvalue)))))

(fn `UserConstructionScript`)